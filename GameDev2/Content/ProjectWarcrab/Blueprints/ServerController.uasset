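; ServerController is a controller for click-to-move movement and weapon firing, commented as networked movement.
; MoveToHitLocation issues MoveToLocation toward the hit point, ignoring clicks closer than MinClickDistance.
; BeginPlay adds a HUD widget to the viewport.
; FireWeapon is a stub that prints a debug string and stops movement; the missile spawn and aim-rotation nodes are disconnected.
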(event `MoveToHitLocation`
  (params (Hit :type "HitResult Structure"))
  (bind (_bblockinghit _binitialoverlap _time _location) (`GameplayStatics.BreakHitResult` Hit))
  ;[1 1 1] Networked Movement.
  (if (>= (`KismetMathLibrary.VSize` (- (`self.K2_GetActorLocation`) _location)) (`self.minClickDistance`))
    (`self.MoveToLocation` _location)))

(event `self.ReceiveBeginPlay`
  (bind _returnvalue (`|CreateWidget` "/Game/ProjectWarcrab/Blueprints/HUD.HUD_C"))
  (`UserWidget.AddToViewport` _returnvalue 0))

(event `self.ReceiveTick`
  (params (DeltaSeconds :type "Float (single-precision)")))

(event `FireWeapon`
  (params (target_point :type "HitResult Structure"))
  ;[1 1 1] Logic for firing a spell
  (`KismetSystemLibrary.PrintString` "Hello")
  (`self.StopMovement`))

(fn `UserConstructionScript`)