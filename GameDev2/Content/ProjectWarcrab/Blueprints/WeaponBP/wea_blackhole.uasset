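; Black hole weapon actor that drags bots within its radius toward its center.
; Every tick it gathers all Paw_BotProxy actors and passes each in-range ControlledBot to SuckBot.
; SuckBot uses VInterpTo and a swept SetActorLocation to move the bot to the hole's X and Y while keeping its Z.
; Interp speed scales linearly with depth inside the radius, so the pull strengthens toward the center.
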(event `self.ReceiveBeginPlay`)

(event `self.ReceiveActorBeginOverlap`
  (params (OtherActor :type "Actor Object Reference")))

(event `HoleBehavior`
  (params (DT :type "Float (double-precision)"))
  (bind _outactors (`GameplayStatics.GetAllActorsOfClass` "/Game/ProjectWarcrab/Blueprints/paw_BotProxy.paw_BotProxy_C"))
  (for _array_element _outactors
    (bind _controlledbot (`/Game/ProjectWarcrab/Blueprints/paw_BotProxy.ControlledBot` _array_element))
    (bind _returnvalue (- (`self.Radius`) (`self.GetDistanceTo` _controlledbot)))
    ;[1 1 1] If actor to edge is negative, then it is outside the radius
    (if (>= _returnvalue 0.0)
      (`self.SuckBot` _controlledbot DT _returnvalue))))

(event `self.ReceiveTick`
  (params (DeltaSeconds :type "Float (single-precision)"))
  (`self.HoleBehavior` DeltaSeconds))

(fn `SuckBot`
  (params (TargetBot :type "/Game/ProjectWarcrab/Blueprints/cha_BaseBot Object Reference") (DT :type "Float (double-precision)") (RadminDist :type "Float (double-precision)"))
  (bind _returnvalue (`self.K2_GetActorLocation` TargetBot))
  (`self.K2_SetActorLocation` TargetBot (`KismetMathLibrary.VInterpTo` _returnvalue (`KismetMathLibrary.MakeVector` (.x (`self.K2_GetActorLocation`)) (.y (`self.K2_GetActorLocation`)) (.z _returnvalue)) DT (* (/ RadminDist (`self.Radius`)) 10.0)) true false))

(fn `UserConstructionScript`)