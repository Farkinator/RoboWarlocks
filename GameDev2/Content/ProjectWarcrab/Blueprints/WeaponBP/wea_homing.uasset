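; Homing projectile weapon actor that steers toward nearby bots, replicates, and destroys itself after a fixed lifetime.
; Each tick, FindClosest searches Paw_BotProxy actors for the nearest controlled bot within range, excluding the owner.
; HomeRotate then turns toward it at a constant rate, and FlyForward makes a swept move by a fixed per-frame step, independent of delta time.
; Capsule and sphere hit and overlap events only print debug text, with no damage logic.
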(event `self.ReceiveBeginPlay`
  (bind _outactors (`GameplayStatics.GetAllActorsOfClass` "/Game/ProjectWarcrab/Blueprints/cha_BaseBot.cha_BaseBot_C"))
  (set `self.targets` _outactors)
  (`self.SetReplicates` true)
  (`ActorComponent.SetIsReplicated` (`self.DefaultSceneRoot`) true)
  (`KismetSystemLibrary.Delay` 7.0)
  (`self.K2_DestroyActor`))

(event `self.ReceiveActorBeginOverlap`
  (params (OtherActor :type "Actor Object Reference")))

(event `HomingBehavior`
  (params (DT :type "Float (double-precision)"))
  (bind _closest (`self.FindClosest`))
  (if (`self.homing`)
    (`self.HomeRotate` _closest DT))
  (`self.FlyForward`)
  (set `self.closest` -1.0)
  (set `self.homing` false))

(event `self.ReceiveTick`
  (params (DeltaSeconds :type "Float (single-precision)"))
  (`self.HomingBehavior` DeltaSeconds))

(event `self.Capsule.OnComponentHit`
  (params (OtherActor :type "Actor Object Reference") (OtherComp :type "PrimitiveComponent Object Reference") (NormalImpulse :type "Vector Structure") (Hit :type "HitResult Structure (by ref)"))
  (`KismetSystemLibrary.PrintString` "Homing Cap Hit"))

(event `self.Capsule.OnComponentBeginOverlap`
  (params (OtherActor :type "Actor Object Reference") (OtherComp :type "PrimitiveComponent Object Reference") (OtherBodyIndex :type Integer) (bFromSweep :type Boolean) (SweepResult :type "HitResult Structure (by ref)"))
  (`KismetSystemLibrary.PrintString` "Homing Cap Overlap"))

(event `self.Sphere.OnComponentHit`
  (params (OtherActor :type "Actor Object Reference") (OtherComp :type "PrimitiveComponent Object Reference") (NormalImpulse :type "Vector Structure") (Hit :type "HitResult Structure (by ref)"))
  (`KismetSystemLibrary.PrintString` "Homing Hit"))

(event `self.Sphere.OnComponentBeginOverlap`
  (params (OtherActor :type "Actor Object Reference") (OtherComp :type "PrimitiveComponent Object Reference") (OtherBodyIndex :type Integer) (bFromSweep :type Boolean) (SweepResult :type "HitResult Structure (by ref)"))
  (`KismetSystemLibrary.PrintString` "Homing Overlap"))

(fn `FindClosest`
  (returns (Closest :type "/Game/ProjectWarcrab/Blueprints/cha_BaseBot Object Reference"))
  (bind _closest (`self.closest`))
  (bind _outactors (`GameplayStatics.GetAllActorsOfClass` "/Game/ProjectWarcrab/Blueprints/paw_BotProxy.paw_BotProxy_C"))
  (for _array_element _outactors
    (bind _controlledbot (`/Game/ProjectWarcrab/Blueprints/paw_BotProxy.ControlledBot` _array_element))
    (bind _returnvalue (`self.GetDistanceTo` _controlledbot))
    ;[1 1 1] Check if in range of rocket
    (if (<= _returnvalue (`self.Range`))
      ;[1 1 1] Check if there is a closest, and if it is closer
      (if (and (or (< _closest 0.0) (< _returnvalue _closest)) (!= _controlledbot (`self.GetOwner`)))
        (set `self.closestbot` _controlledbot)
        (set `self.homing` true)
        (set `self.closest` _returnvalue))))
  (return (`self.closestbot`)))

(fn `FlyForward`
  (`self.K2_SetActorLocation` (+ (* (`KismetMathLibrary.GetForwardVector` (`self.K2_GetActorRotation`)) 15.0) (`self.K2_GetActorLocation`)) true))

(fn `HomeRotate`
  (params (targetbot :type "/Game/ProjectWarcrab/Blueprints/cha_BaseBot Object Reference") (dT :type "Float (double-precision)"))
  (`self.SetActorRotation` (`KismetMathLibrary.RInterpTo_Constant` (`self.K2_GetActorRotation`) (`KismetMathLibrary.FindLookAtRotation` (`self.K2_GetActorLocation`) (`self.K2_GetActorLocation` targetbot)) dT 90.0)))

(fn `UserConstructionScript`)