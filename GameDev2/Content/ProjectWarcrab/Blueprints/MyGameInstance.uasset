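; Game instance that drives front-end menu flow and multiplayer session hosting, joining and teardown.
; A state machine macro hides the outgoing screen or destroys the session when leaving gameplay, then show events lazily create and cache their widgets with UI-only input.
; Hosting validates the game name, creates an Advanced Sessions session and opens the map as a listen server.
; Session failures destroy the session and show an error dialog.
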(event `ShowCreateLobbyUI`
  (bind _returnvalue (`GameplayStatics.GetPlayerController` 0))
  ;[1 1 1] Sets Up the Lobby Creation UI
  (`self.TransitionToState` "NewEnumerator7"
    (:`NewState`
      (`/Engine/EditorBlueprintResources/StandardMacros.IsValid` (`self.LobbyCreation`)
        (:`Is Valid`
          _)
        (:`Is Not Valid`
          (bind _returnvalue_2 (`|CreateWidget` "/Game/ProjectWarcrab/Blueprints/Widgets/LobbyCreation.LobbyCreation_C" _returnvalue))
          (bind _output_get (set `self.LobbyCreation` _returnvalue_2))))
      (`UserWidget.AddToViewport` _output_get 0)
      (`WidgetBlueprintLibrary.SetInputMode_UIOnlyEx` _returnvalue _output_get))))

(event `ShowServerList`
  (bind _returnvalue (`GameplayStatics.GetPlayerController` 0))
  ;[1 1 1] Show Server List when clicked from main menu
  (`self.TransitionToState` "NewEnumerator5"
    (:`SameState`
      _)
    (:`NewState`
      (`/Engine/EditorBlueprintResources/StandardMacros.IsValid` (`self.ServerList`)
        (:`Is Valid`
          _)
        (:`Is Not Valid`
          (bind _returnvalue_2 (`|CreateWidget` "/Game/ProjectWarcrab/Blueprints/Widgets/ServerList.ServerList_C" _returnvalue))
          (bind _output_get (set `self.ServerList` _returnvalue_2))))))
  (`UserWidget.AddToViewport` _output_get 0)
  (`WidgetBlueprintLibrary.SetInputMode_UIOnlyEx` _returnvalue _output_get))

(event `ShowMainMenuEvent`
  (bind _returnvalue (`GameplayStatics.GetPlayerController` 0))
  ;[1 1 1] Show the Main Menu.
  (`self.IsCurrentState` "NewEnumerator4"
    (:`true`
      (`GameplayStatics.OpenLevel` "MainMenu"))
    (:`false`
      _))
  (`self.TransitionToState` "NewEnumerator2"
    (:`NewState`
      (`/Engine/EditorBlueprintResources/StandardMacros.IsValid` (`self.MainMenu`)
        (:`Is Valid`
          _)
        (:`Is Not Valid`
          (bind _returnvalue_2 (`|CreateWidget` "/Game/ProjectWarcrab/Blueprints/Widgets/MainMenu.MainMenu_C" _returnvalue))
          (set `self.MainMenu` _returnvalue_2)))
      (`WidgetBlueprintLibrary.SetInputMode_UIOnlyEx` _returnvalue (`self.MainMenu`))
      (`UserWidget.AddToViewport` (`self.MainMenu`) 0))))

(event `HostGameEvent`
  (params (GameName :type String) (NumPlayers :type Integer))
  ;[1 1 1] Host a Game Session
  (bind _lobbysettings (`self.CreateLobbySettings` GameName)
    (:`Success`
      (`CreateSessionCallbackProxyAdvanced.CreateAdvancedSession` _lobbysettings (`GameplayStatics.GetPlayerController` 0) NumPlayers 0 (`self.LANenabled`)
        (:`OnSuccess`
          (`GameplayStatics.OpenLevel` "TopDownExampleMap" true "listen")
          (set `self.maxPlayers` NumPlayers))
        (:`OnFailure`
          (`self.DisplayErrorDialog` "Error: Could Not create session"))))))

(event `JoinFromServerList`
  (params (searchResult :type "BlueprintSessionResult Structure"))
  ;[1 1 1] Join from serverlist.
  (`JoinSessionCallbackProxy.JoinSession` (`GameplayStatics.GetPlayerController` 0) searchResult
    (:`OnSuccess`
      (set `self.maxPlayers` (`FindSessionsCallbackProxy.GetMaxPlayers` searchResult)))
    (:`OnFailure`
      (`self.DisplayErrorDialog` "Error: Could not join session"))))

(event `DestroySessionCaller`
  ;[1 1 1] Destroys this session (Disconnect)
  (`DestroySessionCallbackProxy.DestroySession` (`GameplayStatics.GetPlayerController` 0)))

(fn `GameStartup`
  (`self.IsCurrentState` "NewEnumerator0"
    (:`true`
      (`self.ShowMainMenuEvent`))))

(fn `HideWidget`
  (params (Widget :type "Widget Object Reference"))
  (`Widget.RemoveFromParent` Widget))

(fn `StartLobbyState`
  (`self.TransitionToState` "NewEnumerator6"))

(fn `StartPlayingState`
  (`self.TransitionToState` "NewEnumerator4"))