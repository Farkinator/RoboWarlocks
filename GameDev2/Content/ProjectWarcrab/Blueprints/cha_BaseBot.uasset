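; Base bot character that moves toward right-click hits, fires weapons, can be launched and shows a fire effect.
; Movement uses direct movement input beyond a minimum click distance; the AI MoveToLocation path is unwired.
; FireWeapon stops movement, interpolates one yaw step toward the target, then spawns a basic or homing missile by slot.
; LaunchBot applies a lofted impulse, Tick syncs fire particles to OnFire, and BeginPlay replicates camera components.
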(event `ClientRightClick`
  (params (destination :type "HitResult Structure"))
  (`self.MoveToHitLocation` destination))

(event `self.ReceiveBeginPlay`
  (`ActorComponent.SetIsReplicated` (`self.SpringArm`) true)
  (`ActorComponent.SetIsReplicated` (`self.Camera`) true))

(event `self.ReceiveTick`
  (params (DeltaSeconds :type "Float (single-precision)"))
  (`self.CheckFire`))

(fn `CheckFire`
  (bind _particlesystem (`self.ParticleSystem`))
  (if (`self.onFire`)
    (`ActorComponent.Activate` _particlesystem false)
    (`SceneComponent.K2_SetRelativeRotation` (`self.ParticleSystem`) (`self.K2_GetActorRotation`) false false)
    (else
      (`ActorComponent.Deactivate` _particlesystem))))

(fn `FireWeapon`
  (params (WeaponTarget :type "HitResult Structure") (weapon_slot :type Integer))
  (bind _returnvalue (`self.K2_GetActorRotation`))
  (bind _returnvalue_2 (`KismetMathLibrary.MakeTransform` (+ (.location (`SceneComponent.K2_GetComponentToWorld` (`self.Mesh`))) (* (`KismetMathLibrary.GetForwardVector` _returnvalue) 100.0)) (.rotation (`SceneComponent.K2_GetComponentToWorld` (`self.Mesh`))) (1.0 1.0 1.0)))
  (`KismetSystemLibrary.PrintString` "Hello")
  (`MovementComponent.StopMovementImmediately` (`self.CharacterMovement`)) ; stop movement, play cast animation
  (`self.SetActorRotation` (`KismetMathLibrary.RInterpTo` _returnvalue (`KismetMathLibrary.MakeRotator` 0.0 0.0 (.yaw (`KismetMathLibrary.FindLookAtRotation` (`self.K2_GetActorLocation` self) (`.Location` (`GameplayStatics.BreakHitResult` WeaponTarget))))) (`GameplayStatics.GetWorldDeltaSeconds`) (.yaw (`CharacterMovementComponent.RotationRate` (`self.CharacterMovement`)))))
  ;[1 1 1] Spawn the projectile where it needs to go.
  (switch `int` weapon_slot
    (:`Default`
      (`|SpawnActorFromClass` "/Game/ProjectWarcrab/Blueprints/WeaponBP/wea_BasicMissile.wea_BasicMissile_C" _returnvalue_2 "Undefined" "OverrideRootScale" null self :!label _label))
    (:`1`
      (goto _label))
    (:`2`
      (`|SpawnActorFromClass` "/Game/ProjectWarcrab/Blueprints/WeaponBP/wea_homing.wea_homing_C" _returnvalue_2 "Undefined" "OverrideRootScale" null self :!label _label_2))
    (:`3`
      (goto _label_2))
    (:`4`
      (goto _label_2))))

(fn `LaunchBot`
  (params (Direction :type "Vector Structure") (Magnitude :type "Float (double-precision)"))
  (`NavMovementComponent.StopActiveMovement` (`self.CharacterMovement`))
  (`self.LaunchCharacter` (* (* (`KismetMathLibrary.MakeVector` (.x (`KismetMathLibrary.Normal` Direction)) (.y (`KismetMathLibrary.Normal` Direction)) 0.25) 10.0) Magnitude)))

(fn `MoveToHitLocation`
  (params (Hit :type "HitResult Structure"))
  (bind _returnvalue (`self.K2_GetActorLocation`))
  (bind (_bblockinghit _binitialoverlap _time _location) (`GameplayStatics.BreakHitResult` Hit))
  (bind _returnvalue_2 (`KismetMathLibrary.VSize` (- _returnvalue _location)))
  (if (>= _returnvalue_2 (`self.minClickDistance`))
    (`self.AddMovementInput` (`KismetMathLibrary.GetDirectionVector` _returnvalue _location) _returnvalue_2)))

(fn `TargetWeapon`
  (params (weapon_slot :type Integer))
  (returns (weapon_exists :type Boolean))
  ;[1 1 1] Returns if this slot has a weapon attached to it.
  (return (!= (`KismetArrayLibrary.Array_Get` (`self.weaponarray`) weapon_slot) 0)))

(fn `UserConstructionScript`)