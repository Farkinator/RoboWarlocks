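; Proxy pawn that stands in for a server-controlled bot character.
; On BeginPlay, the authority spawns a Cha_BaseBot and a ServerController at the proxy's transform, and that AI controller possesses the bot.
; Each tick, while the bot is valid, the proxy moves halfway toward the bot's transform, giving smoothed but frame-rate-dependent following.
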(event `self.ReceiveBeginPlay`
  (bind _returnvalue (`self.GetTransform`))
  ;[1 1 1] Spawn the actual character, and an AI controller that will control the character server-side
  (`/Engine/EditorBlueprintResources/ActorMacros.Switch Has Authority`
    (:`Authority`
      (bind _returnvalue_2 (`|SpawnActorFromClass` "/Game/ProjectWarcrab/Blueprints/cha_BaseBot.cha_BaseBot_C" _returnvalue "Undefined" "OverrideRootScale"))
      (set `self.ControlledBot` _returnvalue_2)
      (bind _returnvalue_3 (`|SpawnActorFromClass` "/Game/ProjectWarcrab/Blueprints/ServerController.ServerController_C" _returnvalue "Undefined" "OverrideRootScale"))
      (set `self.ServerSideController` _returnvalue_3)
      (`Controller.Possess` (`self.ServerSideController`) (`self.ControlledBot`)))))

(event `self.ReceiveTick`
  (params (DeltaSeconds :type "Float (single-precision)"))
  (bind _controlledbot (`self.ControlledBot`))
  ;[1 1 1] Update our proxy controller
  (`/Engine/EditorBlueprintResources/StandardMacros.IsValid` _controlledbot
    (:`Is Valid`
      (`self.K2_SetActorTransform` (`KismetMathLibrary.TLerp` (`self.GetTransform` _controlledbot) (`self.GetTransform`) 0.5)))))

(fn `UserConstructionScript`)