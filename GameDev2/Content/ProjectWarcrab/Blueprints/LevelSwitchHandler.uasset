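; LevelSwitchHandler is an actor that handles level switches and the loading-screen widgets shown around them.
; On BeginPlay, if the load-in flag is set, it displays a MainMenu widget as the loading screen, then removes it once a timer counted down in Tick expires.
; NextLevel shows a ServerRow widget and opens the level by the name stored through SetNextLevel.
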(event `self.ReceiveBeginPlay`
  (if (`self.bool_LoadIn`)
    (bind _returnvalue (`|CreateWidget` "/Game/ProjectWarcrab/Blueprints/Widgets/MainMenu.MainMenu_C"))
    (bind _output_get (set `self.wid_LoadingScreen` _returnvalue))
    (bind _asuser_widget (cast `UserWidget` _output_get))
    (`UserWidget.AddToViewport` _asuser_widget 1)))

(event `self.ReceiveActorBeginOverlap`
  (params (OtherActor :type "Actor Object Reference")))

(event `self.ReceiveTick`
  (params (DeltaSeconds :type "Float (single-precision)"))
  (bind _flt_loadtime (`self.flt_LoadTime`))
  (if (> _flt_loadtime 0.0)
    (set `self.flt_LoadTime` (- _flt_loadtime DeltaSeconds))
    (elif (`self.bool_LoadIn`)
      (set `self.bool_LoadIn` false)
      (`Widget.RemoveFromParent` (`self.wid_LoadingScreen`)))))

(fn `NextLevel`
  (bind _returnvalue (`|CreateWidget` "/Game/ProjectWarcrab/Blueprints/Widgets/ServerRow.ServerRow_C"))
  (bind _output_get (set `self.wid_LoadingScreen` _returnvalue))
  (bind _asuser_widget (cast `UserWidget` _output_get))
  (`UserWidget.AddToViewport` _asuser_widget 0)
  (`GameplayStatics.OpenLevel` (`KismetStringLibrary.Conv_StringToName` (`self.str_NextLevel`))))

(fn `SetNextLevel`
  (params (name_NextLevel :type String))
  (set `self.str_NextLevel` name_NextLevel))

(fn `UserConstructionScript`)