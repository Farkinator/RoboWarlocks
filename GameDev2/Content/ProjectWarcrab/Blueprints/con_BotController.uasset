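; Player controller for a click-controlled bot, handling weapon targeting, firing and movement through a paw_BotProxy pawn.
; Weapon keys enable targeting, but a hard-coded false branch then resets the selected slot to -1; left click calls FireWeapon on the proxy's ControlledBot.
; Right click cancels targeting or sends the cursor hit to the proxy's ServerSideController.
; Tick traces below the pawn, printing a lava warning outside safezone material except in MainMenu.
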(event `InputAction|LeftClick`
  (params (Key :type "Key Structure" :default "AnyKey"))
  (:`Pressed`
    (if (`self.targetingOn`)
      (`self.EventFireWeapon` (`self.GetHitResultUnderCursorByChannel` "TraceTypeQuery1"))
      (set `self.targetingOn` false))))

(event `InputAction|SetDestination`
  (params (Key :type "Key Structure" :default "AnyKey"))
  ;[1 1 1] Click and go there
  (:`Pressed`
    (if (`self.targetingOn`)
      (set `self.targetingOn` false)
      (else
        (`self.EventMoveToLocation` (`self.GetHitResultUnderCursorByChannel` "TraceTypeQuery1"))))))

(event `EventFireWeapon`
  (params (WeaponTarget :type "HitResult Structure"))
  ;[1 1 1] If we're targeting, then fire the weapon that is selected.
  (bind _aspaw_bot_proxy (cast `/Game/ProjectWarcrab/Blueprints/paw_BotProxy` (`self.K2_GetPawn` self)))
  (`/Game/ProjectWarcrab/Blueprints/cha_BaseBot.FireWeapon` (`/Game/ProjectWarcrab/Blueprints/paw_BotProxy.ControlledBot` _aspaw_bot_proxy) WeaponTarget (`self.WeaponSelected`)))

(event `EventMoveToLocation`
  (params (Destination :type "HitResult Structure"))
  ;[1 1 1] This only runs on the server, because only the server has the nav grid.
  (bind _aspaw_bot_proxy (cast `/Game/ProjectWarcrab/Blueprints/paw_BotProxy` (`self.K2_GetPawn` self)))
  (`/Game/ProjectWarcrab/Blueprints/ServerController.MoveToHitLocation` (`/Game/ProjectWarcrab/Blueprints/paw_BotProxy.ServerSideController` _aspaw_bot_proxy) Destination))

(event `InputAction|Weapon0`
  (params (Key :type "Key Structure" :default "AnyKey"))
  ;[1 1 1] If the player hits a weapon button, turn on the targeting ui.
  (:`Pressed`
    (set `self.WeaponSelected` 0)
    (set `self.targetingOn` true :!label _label) ; we'll be targeting stuff if the weapon exists.
    (if false
      (`self.EventTargetWeapon`)
      (else
        (set `self.WeaponSelected` -1)))))

(event `EventTargetWeapon`)

(event `InputAction|Weapon1`
  (params (Key :type "Key Structure" :default "AnyKey"))
  ;[1 1 1] If the player hits a weapon button, turn on the targeting ui.
  (:`Pressed`
    (set `self.WeaponSelected` 1)
    (goto _label)))

(event `InputAction|Weapon2`
  (params (Key :type "Key Structure" :default "AnyKey"))
  ;[1 1 1] If the player hits a weapon button, turn on the targeting ui.
  (:`Pressed`
    (set `self.WeaponSelected` 2)
    (goto _label)))

(event `InputAction|Weapon3`
  (params (Key :type "Key Structure" :default "AnyKey"))
  ;[1 1 1] If the player hits a weapon button, turn on the targeting ui.
  (:`Pressed`
    (set `self.WeaponSelected` 3)
    (goto _label)))

(event `self.ReceiveTick`
  (params (DeltaSeconds :type "Float (single-precision)"))
  (bind _returnvalue (`self.K2_GetActorLocation` (`self.K2_GetPawn`)))
  (bind _outhit (`KismetSystemLibrary.LineTraceSingle` _returnvalue (- _returnvalue (0.0 0.0 100.0)) "TraceTypeQuery1"))
  (bind _returnvalue_2 (`GameplayStatics.GetCurrentLevelName` true))
  (if (and (!= _returnvalue_2 "MainMenu") (!= (`KismetStringLibrary.Conv_ObjectToString` (`.PhysMat` (`GameplayStatics.BreakHitResult` _outhit))) "safezone"))
    (`KismetSystemLibrary.PrintString` "LAVA!")))

(fn `FireWeapon`
  (params (SpellTarget :type "HitResult Structure")))

(fn `MoveToHitLocation`
  (params (Hit :type "HitResult Structure"))
  (bind _returnvalue (`self.K2_GetPawn`))
  (bind (_bblockinghit _binitialoverlap _time _location) (`GameplayStatics.BreakHitResult` Hit))
  (bind _returnvalue_2 (`self.K2_GetActorLocation` _returnvalue))
  (bind _returnvalue_3 (`KismetMathLibrary.VSize` (- _returnvalue_2 _location)))
  (if (>= _returnvalue_3 (`self.minClickDistance`))
    (`Pawn.AddMovementInput` _returnvalue (`KismetMathLibrary.GetDirectionVector` _returnvalue_2 _location) _returnvalue_3 false)))

(fn `OnRep_targetingOn`)

(fn `UserConstructionScript`)